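; BP_CellBonus is a cell Blueprint that awards bonus score to the player who triggers it.
; Its Action override calls the parent, then shows a WB_Bonus widget on screen.
; It adds the cell's Score to that player's total in BP_GameMode, treating any non-zero PlayerId as player 1, and prints the new total.
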(fn `Action`
  (params (PlayerId :type Integer))
  (`parent.Action` PlayerId)
  (if (== PlayerId 0)
    (bind _returnvalue (`|CreateWidget` "/Game/Blueprints/Widget/WB_Bonus.WB_Bonus_C"))
    (`UserWidget.AddToViewport` _returnvalue 0)
    (bind _asbp_game_mode (cast `/Game/Blueprints/BP_GameMode` (`GameplayStatics.GetGameMode`)))
    (bind _output_get (set `/Game/Blueprints/BP_GameMode.ScoreTotalPlayer0` (+ (`/Game/Blueprints/BP_GameMode.ScoreTotalPlayer0` _asbp_game_mode) (`self.Score`)) _asbp_game_mode))
    (`KismetSystemLibrary.PrintString` (`KismetStringLibrary.Conv_IntToString` _output_get))
    (else
      (bind _returnvalue_2 (`|CreateWidget` "/Game/Blueprints/Widget/WB_Bonus.WB_Bonus_C"))
      (`UserWidget.AddToViewport` _returnvalue_2 0)
      (bind _asbp_game_mode_2 (cast `/Game/Blueprints/BP_GameMode` (`GameplayStatics.GetGameMode`)))
      (bind _output_get_2 (set `/Game/Blueprints/BP_GameMode.ScoreTotalPlayer1` (+ (`/Game/Blueprints/BP_GameMode.ScoreTotalPlayer1` _asbp_game_mode_2) (`self.Score`)) _asbp_game_mode_2))
      (`KismetSystemLibrary.PrintString` (`KismetStringLibrary.Conv_IntToString` _output_get_2)))))

(fn `UserConstructionScript`
  (`parent.UserConstructionScript`))