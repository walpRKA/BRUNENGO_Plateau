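; BP_Tile is a Mahjong-themed tile actor, apparently for a memory game, with a face mesh called Recto.
; On BeginPlay, ChangeCardColor switches over eight face types to set the matching material, but its selector is fixed at White, so the white face always applies.
; ToggleCard is an empty stub; the nodes that would flip the root 180 degrees in roll are disconnected and never run.
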(event `self.ReceiveBeginPlay`
  (`self.ChangeCardColor`))

(fn `ChangeCardColor`
  (switch `/Game/Blueprints/Memory/TileType` "NewEnumerator0"
    (:`NewEnumerator0`
      (`PrimitiveComponent.SetMaterial` (`self.Recto`) 0 "/Game/Blueprints/Memory/materials/MI/mahjong_blanc_Mat_Inst.mahjong_blanc_Mat_Inst"))
    (:`NewEnumerator1`
      (`PrimitiveComponent.SetMaterial` (`self.Recto`) 0 "/Game/Blueprints/Memory/materials/MI/mahjong_rouge_Mat_Inst.mahjong_rouge_Mat_Inst"))
    (:`NewEnumerator2`
      (`PrimitiveComponent.SetMaterial` (`self.Recto`) 0 "/Game/Blueprints/Memory/materials/MI/mahjong_vert_Mat_Inst.mahjong_vert_Mat_Inst"))
    (:`NewEnumerator3`
      (`PrimitiveComponent.SetMaterial` (`self.Recto`) 0 "/Game/Blueprints/Memory/materials/MI/mahjong_pin_Mat_Inst.mahjong_pin_Mat_Inst"))
    (:`NewEnumerator4`
      (`PrimitiveComponent.SetMaterial` (`self.Recto`) 0 "/Game/Blueprints/Memory/materials/MI/mahjong_bamboo_Mat_Inst.mahjong_bamboo_Mat_Inst"))
    (:`NewEnumerator5`
      (`PrimitiveComponent.SetMaterial` (`self.Recto`) 0 "/Game/Blueprints/Memory/materials/MI/majong_chiffre_Mat_Inst.majong_chiffre_Mat_Inst"))
    (:`NewEnumerator6`
      (`PrimitiveComponent.SetMaterial` (`self.Recto`) 0 "/Game/Blueprints/Memory/materials/MI/mahjong_nord_Mat_Inst.mahjong_nord_Mat_Inst"))
    (:`NewEnumerator7`
      (`PrimitiveComponent.SetMaterial` (`self.Recto`) 0 "/Game/Blueprints/Memory/materials/MI/mahjong_est_Mat_Inst.mahjong_est_Mat_Inst"))))

(fn `ToggleCard`)

(fn `UserConstructionScript`)