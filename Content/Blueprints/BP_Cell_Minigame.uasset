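; BP_Cell_Minigame is a cell whose action sends the player who triggers it into a randomly chosen minigame.
; It overrides Action to store the player ID in BP_GameInstance, then calls the parent Action with a fixed ID rather than the one received.
; It adds a WB_Minigame widget to the viewport and opens either CollectMap or MemoryMap based on a random boolean.
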(fn `Action`
  (params (PlayerId :type Integer))
  (bind _asbp_game_instance (cast `/Game/Blueprints/BP_GameInstance` (`GameplayStatics.GetGameInstance`)))
  (`/Game/Blueprints/BP_GameInstance.RememberMinigamePlayer` _asbp_game_instance PlayerId)
  (`parent.Action` 0)
  (bind _returnvalue (`|CreateWidget` "/Game/Blueprints/Widget/WB_Minigame.WB_Minigame_C"))
  (`UserWidget.AddToViewport` _returnvalue 0)
  (if (`KismetMathLibrary.RandomBool`)
    (`GameplayStatics.OpenLevelBySoftObjectPtr` "/Game/Maps/CollectMap.CollectMap")
    (else
      (`GameplayStatics.OpenLevelBySoftObjectPtr` "/Game/Maps/MemoryMap.MemoryMap"))))

(fn `UserConstructionScript`
  (`parent.UserConstructionScript`))