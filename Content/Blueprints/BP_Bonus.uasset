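; BP_Bonus is a child Blueprint that awards a 100-point bonus when its Action runs for a player.
; The Action override calls the parent, passes CurrentScore through a temporary SPlayerData struct, adds the bonus, stores it back in CurrentScore and prints it.
; The event graph is only disabled placeholder nodes, and the construction script just calls its parent.
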(fn `Action`
  (params (PlayerId :type Integer))
  (`parent.Action` PlayerId)
  (bind _output_get (set `self.CurrentScore` (+ (`.Score_4_09C81F4044D8FFB79AE82DA3832970A2` (break `/Game/Blueprints/S_PlayerData` (make `/Game/Blueprints/S_PlayerData` PlayerId (`self.CurrentScore`)))) 100)))
  (`KismetSystemLibrary.PrintString` (`KismetStringLibrary.Conv_IntToString` _output_get)))

(fn `UserConstructionScript`
  (`parent.UserConstructionScript`))