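; Game mode for a single-player dice board game that spawns the pawn and die and runs each roll-and-move turn.
; After a short delay, BeginPlay places the pawn on player 0's cell stored in the GI_Board game instance.
; RollDiceAndMove saves the new cell index, wrapping only when already at the last cell, and moves the pawn.
; A pawn location matching a hard-coded cell shows WB_END and destroys both actors.
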(event `self.ReceiveBeginPlay`
  (`KismetSystemLibrary.Delay` 0.2)
  (bind _asgi_board (cast `/Game/Blueprint/GI_Board` (`GameplayStatics.GetGameInstance`)))
  (bind _output_get (set `self.As GI Board` _asgi_board))
  (bind _playercellnumber (`/Game/Blueprint/GI_Board.GetPlayerCellNumberByPlayerID` _output_get 0))
  (bind _returnvalue_location (`self.GetCellPositionByNumber` (`self.BP_Board`) _playercellnumber))
  (bind _returnvalue (`|SpawnActorFromClass` "/Game/Blueprint/BP_Pion.BP_Pion_C" (`KismetMathLibrary.MakeTransform` _returnvalue_location) "Undefined" "MultiplyWithRoot" null null))
  (set `self.BP_Pion` _returnvalue)
  (bind _returnvalue_2 (`|SpawnActorFromClass` "/Game/Blueprint/BP_Des.BP_Des_C" (`KismetMathLibrary.MakeTransform` (0.0 0.0 0.0)) "Undefined" "MultiplyWithRoot" null null))
  (set `self.BP_Des` _returnvalue_2))

(fn `GetCellPositionByNumber`
  (params (BP_Board :type "/Game/Blueprint/BP_Board Object Reference") (`Cell Index` :type Integer))
  (returns (ReturnValue_Location :type "Vector Structure"))
  (bind _output_get (set `self.BP_Board` BP_Board))
  (bind _output (`|GetArrayItem` (`/Game/Blueprint/BP_Board.BP_Cell` _output_get) `Cell Index`))
  (`KismetSystemLibrary.PrintString` (`KismetSystemLibrary.GetDisplayName` _output))
  (bind _returnvalue_location (`KismetMathLibrary.BreakTransform` (`self.GetTransform` _output)))
  (return _returnvalue_location))

(fn `RollDiceAndMove`
  (bind _bp_des (`self.BP_Des`))
  (bind _bp_cell (`/Game/Blueprint/BP_Board.BP_Cell` (`self.BP_Board`)))
  (`/Game/Blueprint/BP_Des.RollDice` _bp_des)
  (bind _playercellnumber (`/Game/Blueprint/GI_Board.GetPlayerCellNumberByPlayerID` (`self.As GI Board`) 0))
  (if (>= _playercellnumber (- (`KismetArrayLibrary.Array_Length` _bp_cell) 1))
    (bind _returnvalue (- (+ _playercellnumber (`/Game/Blueprint/BP_Des.ActualDiceResult` (`self.BP_Des`))) (- (`KismetArrayLibrary.Array_Length` _bp_cell) 1) 0))
    (`/Game/Blueprint/GI_Board.SetPlayerCellNumberByPlayerID` (`self.As GI Board`) 0 _returnvalue)
    (bind _returnvalue_location (`self.GetCellPositionByNumber` (`self.BP_Board`) _returnvalue))
    (`/Game/Blueprint/BP_Pion.MoveToNewCell` (`self.BP_Pion`) _returnvalue_location)
    (else
      (bind _returnvalue_2 (+ _playercellnumber (`/Game/Blueprint/BP_Des.ActualDiceResult` _bp_des)))
      (`/Game/Blueprint/GI_Board.SetPlayerCellNumberByPlayerID` (`self.As GI Board`) 0 _returnvalue_2)
      (bind _returnvalue_location_2 (`self.GetCellPositionByNumber` (`self.BP_Board`) _returnvalue_2))
      (`/Game/Blueprint/BP_Pion.MoveToNewCell` (`self.BP_Pion`) _returnvalue_location_2)))
  (if (== (`self.K2_GetActorLocation` (`self.BP_Pion`)) (`self.K2_GetActorLocation` (`|GetArrayItem` (`/Game/Blueprint/BP_Board.BP_Cell` (`self.BP_Board`)) 14)))
    (bind _returnvalue_3 (`|CreateWidget` "/Game/Blueprint/WB_END.WB_END_C"))
    (`UserWidget.AddToViewport` _returnvalue_3 0)
    (`self.K2_DestroyActor` (`self.BP_Pion`))
    (`self.K2_DestroyActor` (`self.BP_Des`))))

(fn `UserConstructionScript`)