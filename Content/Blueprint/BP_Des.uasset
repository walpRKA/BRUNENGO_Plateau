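; BP_Des is a dice actor that connects the on-screen dice button to the game mode's roll-and-move logic.
; On BeginPlay it caches BP_GameMode, adds a WB_Interface widget to the viewport and binds its DiceButton click to DiceRoll, which calls RollDiceAndMove.
; A separate RollDice function, not called within this Blueprint, prints random rolls in a loop, overwriting the result instead of summing it.
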(event `self.ReceiveBeginPlay`
  (bind _asbp_game_mode (cast `/Game/Blueprint/BP_GameMode` (`GameplayStatics.GetGameMode`)))
  (set `self.As BP Game Mode` _asbp_game_mode)
  (bind _returnvalue (`|CreateWidget` "/Game/Blueprint/WB_Interface.WB_Interface_C"))
  (bind _output_get (set `self.WB_Interface` _returnvalue))
  (`UserWidget.AddToViewport` _output_get 0)
  (add `Button.OnClicked` (`/Game/Blueprint/WB_Interface.DiceButton` (`self.WB_Interface`)) (delegate `DiceRoll`)))

(event `DiceRoll`
  (`/Game/Blueprint/BP_GameMode.RollDiceAndMove` (`self.As BP Game Mode`))
  (`KismetSystemLibrary.PrintString` "je roule les dés"))

(fn `RollDice`
  (set `self.ActualDiceResult` 0)
  (for _ (range (+ (`self.DiceNumber`) 1))
    (bind _output_get (set `self.ActualDiceResult` (`KismetMathLibrary.RandomIntegerInRange` 1 (`self.DiceType`))))
    (`KismetSystemLibrary.PrintString` (`KismetStringLibrary.Conv_IntToString` _output_get) true true (struct :`R` 1.0 :`G` 0.95076 :`A` 1.0))))

(fn `UserConstructionScript`)