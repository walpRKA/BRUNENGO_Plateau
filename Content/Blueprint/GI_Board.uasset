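; GI_Board is a board-game state holder, named as a Game Instance, that tracks each player's cell on the board.
; PlayerList holds SPlayerinfo structs (Player, CellNumber, Score) indexed by PlayerID, with a getter returning that player's cell number.
; The setter calls an array set at that index, but the rebuilt struct carrying the new cell number is shown unconnected to it.
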(fn `GetPlayerCellNumberByPlayerID`
  (params (PlayerID :type Integer))
  (returns (PlayerCellNumber :type Integer))
  (return (`.CellNumber_15_258781C146772C79B74A168ED91ADE79` (break `/Game/Blueprint/S_Playerinfo` (`|GetArrayItem` (`self.PlayerList`) PlayerID)))))

(fn `SetPlayerCellNumberByPlayerID`
  (params (PlayerID :type Integer) (NewCellNumber :type Integer))
  (`KismetArrayLibrary.Array_Set` (`self.PlayerList`) PlayerID))